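; First-person player character with axis-driven walking, controller look and jumping.
; A LockCamera toggle switches between a centered visible cursor in Game and UI input and hidden-cursor Game Only input.
; ComprobarCámara line-traces a short distance from the camera along the control rotation and returns whether the hit actor is a Sensor or Actuador.
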(event Input|ActionEvents|InputActionLockCamera
  (params (Key :type Key%20Structure :default "None"))
  (bind _returnvalue (Game|GetPlayerController 0))
  (bind (_sizex _sizey) (HUD|GetViewportSize _returnvalue))
  ;[1 1 1] Looking Mode
  (:Pressed
    (Utilities|FlowControl|FlipFlop
      (:A
        (Class|PlayerController|SetMouseLocation _returnvalue (/ _sizex 2) (/ _sizey 2))
        (Variables|/Script/Engine.PlayerController|SetbShowMouseCursor _returnvalue true)
        (Input|SetInputModeGameandUI _returnvalue 0 "DoNotLock" true))
      (:B
        (Variables|/Script/Engine.PlayerController|SetbShowMouseCursor _returnvalue false)
        (Input|SetInputModeGameOnly _returnvalue)))))

(event Input|AxisEvents|InputAxisAdelanteAtras
  (params (AxisValue :type Float%20%28single-precision%29))
  ;[0 0 0] Movimiento
  (Pawn|Input|AddMovementInput (Transformation|GetActorForwardVector) AxisValue false))

(event Input|AxisEvents|InputAxisDerechaIzquierda
  (params (AxisValue :type Float%20%28single-precision%29))
  ;[0 0 0] Movimiento
  (Pawn|Input|AddMovementInput (Transformation|GetActorRightVector) AxisValue false))

(event Input|AxisEvents|InputAxisCamaraVertical
  (params (AxisValue :type Float%20%28single-precision%29))
  ;[1 1 1] Control de la cámara
  (Pawn|Input|AddControllerPitchInput AxisValue))

(event Input|AxisEvents|InputAxisCamaraHorizontal
  (params (AxisValue :type Float%20%28single-precision%29))
  ;[1 1 1] Control de la cámara
  (Pawn|Input|AddControllerYawInput AxisValue))

(event Input|KeyboardEvents|SpaceBar
  (params (Key :type Key%20Structure :default "None"))
  ;[0 0.8634 1] Saltar
  (:Pressed
    (Character|Jump))
  (:Released
    (Character|StopJumping)))

(fn ConstructionScript)

(fn ComprobarCámara
  (bind _camera (Variables|Default|GetCamera))
  (bind _returnvalue (Transformation|GetSocketLocation _camera "None"))
  ;[1 1 1] Abrir/Cerrar Persiana
  (bind (_outhit _returnvalue_2) (Collision|LineTraceByChannel _returnvalue (+ _returnvalue (* (Math|Vector|GetForwardVector (Pawn|GetControlRotation :!class /Script/Engine.Pawn)) 7e+02)) "TraceTypeQuery1" false 0 "None"))
  (if _returnvalue_2
    (Utilities|Casting|CastToSensor (.HitActor (Collision|BreakHitResult _outhit))
      (:then
        _)
      (:CastFailed
        (Utilities|Casting|CastToActuador (.HitActor (Collision|BreakHitResult _outhit))
          (:then
            _)
          (:CastFailed
            (return false)))))
    (return true)))
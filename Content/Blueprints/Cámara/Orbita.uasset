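; Orbit camera actor that takes player input to rotate and zoom a view around its position.
; Mouse X yaws the actor, Mouse Y pitches the spring arm, and the wheel scales arm length within clamped limits.
; Left click shows a grab cursor, and E toggles visibility of all actors tagged "Orbita" (walls).
; A trace-based one-by-one wall hiding variant is present but disconnected.
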(event EventBeginPlay
  ;[1 1 1] Guardar modo de juego
  (Input|EnableInput (Game|GetPlayerController 0))
  (bind _asgm_tfg (Utilities|Casting|CastToGM_TFG (Game|GetGameMode)))
  (Variables|Default|SetGame%20Mode _asgm_tfg))

(event Input|MouseEvents|MouseX
  (params (AxisValue :type Float%20%28single-precision%29))
  ;[1 1 1] Mover cámara
  (Class|Actor|AddActorWorldRotation (Math|Rotator|MakeRotator 0.0 0.0 AxisValue)))

(event Input|MouseEvents|MouseY
  (params (AxisValue :type Float%20%28single-precision%29))
  ;[1 1 1] Mover cámara
  (Transformation|AddLocalRotation (Variables|Default|GetSpringArm) (Math|Rotator|MakeRotator 0.0 AxisValue 0.0) false false))

(event Input|MouseEvents|MouseWheelUp
  (params (Key :type Key%20Structure :default "None"))
  (bind _springarm (Variables|Default|GetSpringArm))
  ;[1 1 1] Acercar y alejar la cámara
  (:Pressed
    (Variables|/Script/Engine.SpringArmComponent|SetTargetArmLength _springarm (Math|Float|Clamp(Float) (* (Variables|/Script/Engine.SpringArmComponent|GetTargetArmLength _springarm) 0.9) 5e+02 4e+03))))

(event Input|MouseEvents|MouseWheelDown
  (params (Key :type Key%20Structure :default "None"))
  (bind _springarm (Variables|Default|GetSpringArm))
  ;[1 1 1] Acercar y alejar la cámara
  (:Pressed
    (Variables|/Script/Engine.SpringArmComponent|SetTargetArmLength _springarm (Math|Float|Clamp(Float) (* (Variables|/Script/Engine.SpringArmComponent|GetTargetArmLength _springarm) 1.1) 5e+02 4e+03))))

(event Input|MouseEvents|LeftMouseButton
  (params (Key :type Key%20Structure :default "None"))
  (bind _returnvalue (Game|GetPlayerController 0))
  ;[1 1 1] Cambiar forma cursor
  (:Pressed
    (Variables|/Script/Engine.PlayerController|SetCurrentMouseCursor _returnvalue "GrabHandClosed"))
  (:Released
    (Variables|/Script/Engine.PlayerController|SetCurrentMouseCursor _returnvalue "Default")))

(event Input|KeyboardEvents|E
  (params (Key :type Key%20Structure :default "None"))
  ;[1 1 1] Ocultar todos los muros
  (:Pressed
    (bind _outactors (Actor|GetAllActorswithTag "Orbita"))
    (for _array_element _outactors
      (if (Variables|/Script/Engine.Actor|GetbHidden _array_element)
        (Rendering|SetActorHiddenInGame _array_element false)
        (else
          (Rendering|SetActorHiddenInGame _array_element true))))))

(fn ConstructionScript)